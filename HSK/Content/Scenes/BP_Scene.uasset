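; BP_Scene is a scene that runs the steps in its SceneData in order, currently showing dialogue lines through the dialogue widget.
; On BeginPlay it caches the HSK game mode and, with AutoPlay set, asks it to play the scene.
; The play notification starts the first step.
; Advance skips to the end of a line still playing or moves to the next step; the finished notification is empty.
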(event `self.ReceiveBeginPlay`
  (bind _asbp_hskgame_mode_base (cast `/Game/GameModes/BP_HSKGameModeBase` (`GameplayStatics.GetGameMode`)))
  (set `self.HSKGameMode` _asbp_hskgame_mode_base)
  (`|ExecutionSequence`
    (:`then_0`
      (if (`self.Auto Play`)
        (`HSKGameModeBase.PlayScene` (`self.HSKGameMode`) self)))))

(event `self.NotifyOnPlay`
  (`self.Next Step`))

(event `self.NotifyOnFinished`)

(fn `Advance`
  (bind _dialogue_widget (`/Game/Blueprints/BP_SceneFunctionLibrary.Get Dialogue Widget` self))
  (if (`/Game/UI/WBP_Dialogue.Is Playing` _dialogue_widget)
    (`/Game/UI/WBP_Dialogue.Skip To End Of Line` _dialogue_widget)
    (else
      (`self.Next Step`))))

(fn `Next Step`
  (bind _result (`/Engine/EditorBlueprintResources/StandardMacros.IncrementInt` (`self.Current Step Index`))
    (:`  `
      (`self.Play Step` (`|GetArrayItem` (`HSKSceneData.Steps` (`self.Scene Data`)) _result)))))

(fn `Play Step`
  (params (`Step Info` :type "SceneStep Structure"))
  (bind _step_info_type (break `SceneStep` (`local.Step Info`)))
  (bind (_step_info_type_2 _step_info_dialogueline) (break `SceneStep` (`local.Step Info`)))
  (switch `EStepType` _step_info_type
    (:`DialogueLine`
      (`/Engine/EditorBlueprintResources/StandardMacros.IsValid` _step_info_dialogueline
        (:`Is Valid`
          (`/Game/UI/WBP_Dialogue.Display Line` (`/Game/Blueprints/BP_SceneFunctionLibrary.Get Dialogue Widget` self) (`HSKDialogueDataAsset.DialogueLine` _step_info_dialogueline)))
        (:`Is Not Valid`
          (return))))))

(fn `UserConstructionScript`)